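; Arena floor actor that switches obstacles and a goalkeeper on and off as the player character enters or leaves it.
; Overlap events on its Box trigger respond only to BP_ThirdPersonCharacter.
; Entering sends activate and move messages to the MovingObjects and GoalKeeper references, and leaving sends the matching deactivate and stop messages.
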(event OnComponentBeginOverlap(Box)
  (params (OverlappedComponent :type Primitive%20Component%20Object%20Reference) (OtherActor :type Actor%20Object%20Reference) (OtherComp :type Primitive%20Component%20Object%20Reference) (OtherBodyIndex :type Integer) (bFromSweep :type Boolean) (SweepResult :type Hit%20Result%20Structure%20%28by%20ref%29))
  (Utilities|Casting|CastToBP_ThirdPersonCharacter OtherActor)
  (Class|BPIFunctions|MakeObstacleActive(Message) (Variables|Default|GetMoving_Objects))
  (Class|BPIFunctions|MakeGoalKeeperMove(Message) (Variables|Default|GetGoalKeeper)))

(event OnComponentEndOverlap(Box)
  (params (OverlappedComponent :type Primitive%20Component%20Object%20Reference) (OtherActor :type Actor%20Object%20Reference) (OtherComp :type Primitive%20Component%20Object%20Reference) (OtherBodyIndex :type Integer))
  (Utilities|Casting|CastToBP_ThirdPersonCharacter OtherActor)
  (Class|BPIFunctions|MakeObstacleInactive(Message) (Variables|Default|GetMoving_Objects))
  (Class|BPIFunctions|MakeGoalKeeperUnMove(Message) (Variables|Default|GetGoalKeeper)))

(fn ConstructionScript)