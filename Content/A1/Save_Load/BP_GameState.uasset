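; Game state Blueprint that saves, loads and deletes game progress in a single save slot.
; Save and Checkpoint events load or create a BP_SaveGame object; Save writes red and blue scores, while Checkpoint writes the goal target and player transform.
; Load copies all saved values back into GameInstance_Variables and teleport-free moves the player character to the saved transform.
; Each operation reports its result with on-screen text.
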(event Custom|Save
  ;[1 1 1] Save Game
  (bind _returnvalue (SaveGame|DoesSaveGameExist (Variables|Default|GetSaveSlotName)))
  (if _returnvalue
    (bind _returnvalue_2 (SaveGame|LoadGamefromSlot (Variables|Default|GetSaveSlotName)))
    (bind _output_get (Variables|Default|SetSaveRef _returnvalue_2))
    (CallFunction|SaveGameData _output_get)
    (else
      (bind _returnvalue_3 (SaveGame|CreateSaveGameObject "/Game/A1/Save_Load/BP_SaveGame.BP_SaveGame_C"))
      (bind _output_get_2 (Variables|Default|SetSaveRef _returnvalue_3))
      (CallFunction|SaveGameData _output_get_2))))

(event Custom|Load
  ;[1 1 1] Load Game
  (bind _returnvalue (SaveGame|DoesSaveGameExist (Variables|Default|GetSaveSlotName)))
  (if _returnvalue
    (bind _returnvalue_2 (SaveGame|LoadGamefromSlot (Variables|Default|GetSaveSlotName)))
    (bind _output_get (Variables|Default|SetSaveRef _returnvalue_2))
    (CallFunction|LoadGameData _output_get)
    (else
      (Development|PrintText (Utilities|Text|FormatText "Failed to load data for slot {slotName}" (Variables|Default|GetSaveSlotName))))))

(event Custom|Checkpoint
  ;[1 1 1] Map Checkpoint
  (bind _returnvalue (SaveGame|DoesSaveGameExist (Variables|Default|GetSaveSlotName)))
  (if _returnvalue
    (bind _returnvalue_2 (SaveGame|LoadGamefromSlot (Variables|Default|GetSaveSlotName)))
    (bind _output_get (Variables|Default|SetSaveRef _returnvalue_2))
    (CallFunction|SaveCheckpoint _output_get)
    (else
      (bind _returnvalue_3 (SaveGame|CreateSaveGameObject "/Game/A1/Save_Load/BP_SaveGame.BP_SaveGame_C"))
      (bind _output_get_2 (Variables|Default|SetSaveRef _returnvalue_3))
      (CallFunction|SaveCheckpoint _output_get_2))))

(event Custom|Delete
  (bind _returnvalue (SaveGame|DoesSaveGameExist (Variables|Default|GetSaveSlotName)))
  (if _returnvalue
    (SaveGame|DeleteGameinSlot (Variables|Default|GetSaveSlotName))
    (Development|PrintText "Save data deleted")
    (else
      (Development|PrintText (Utilities|Text|FormatText "Failed to delete data for slot {slotName}" (Variables|Default|GetSaveSlotName))))))

(event EventBeginPlay)

(fn ConstructionScript)

(fn SaveGameData
  (params (Object :type Object%20Object%20Reference))
  (bind _asbp_save_game (Utilities|Casting|CastToBP_SaveGame Object))
  (bind _asgame_instance_variables (Utilities|Casting|CastToGameInstance_Variables (Game|GetGameInstance)))
  (Variables|/Game/A1/Save_Load/BP_SaveGame.BP_SaveGame_C|Setblue_score _asbp_save_game (Variables|/Game/A1/GameInstance_Variables.GameInstance_Variables_C|GetBlue_Score _asgame_instance_variables))
  (Variables|/Game/A1/Save_Load/BP_SaveGame.BP_SaveGame_C|Setred_score _asbp_save_game (Variables|/Game/A1/GameInstance_Variables.GameInstance_Variables_C|GetRed_Score _asgame_instance_variables))
  (bind _returnvalue (SaveGame|SaveGametoSlot (Variables|Default|GetSaveRef) (Variables|Default|GetSaveSlotName)))
  (if _returnvalue
    (Development|PrintText (Utilities|Text|FormatText "Saved data on slot {slotName}" (Variables|Default|GetSaveSlotName)))
    (else
      (Development|PrintText "Error saving file!"))))

(fn LoadGameData
  (params (Object :type Object%20Object%20Reference))
  (bind _asbp_save_game (Utilities|Casting|CastToBP_SaveGame Object))
  (bind _asgame_instance_variables (Utilities|Casting|CastToGameInstance_Variables (Game|GetGameInstance)))
  (Variables|/Game/A1/GameInstance_Variables.GameInstance_Variables_C|SetRed_Score _asgame_instance_variables (Variables|/Game/A1/Save_Load/BP_SaveGame.BP_SaveGame_C|Getred_score _asbp_save_game))
  (Variables|/Game/A1/GameInstance_Variables.GameInstance_Variables_C|SetBlue_Score _asgame_instance_variables (Variables|/Game/A1/Save_Load/BP_SaveGame.BP_SaveGame_C|Getblue_score _asbp_save_game))
  (Variables|/Game/A1/GameInstance_Variables.GameInstance_Variables_C|SetGoal_target _asgame_instance_variables (Variables|/Game/A1/Save_Load/BP_SaveGame.BP_SaveGame_C|Getgoal_target _asbp_save_game))
  (Transformation|SetActorTransform (Game|GetPlayerCharacter 0) (Variables|/Game/A1/Save_Load/BP_SaveGame.BP_SaveGame_C|Getplayer_transform _asbp_save_game))
  (Development|PrintText "Loaded Save Data"))

(fn SaveCheckpoint
  (params (Object :type Object%20Object%20Reference))
  (bind _asbp_save_game (Utilities|Casting|CastToBP_SaveGame Object))
  (bind _asgame_instance_variables (Utilities|Casting|CastToGameInstance_Variables (Game|GetGameInstance)))
  (Variables|/Game/A1/Save_Load/BP_SaveGame.BP_SaveGame_C|Setgoal_target _asbp_save_game (Variables|/Game/A1/GameInstance_Variables.GameInstance_Variables_C|GetGoal_target _asgame_instance_variables))
  (Variables|/Game/A1/Save_Load/BP_SaveGame.BP_SaveGame_C|Setplayer_transform _asbp_save_game (Transformation|GetActorTransform (Game|GetPlayerCharacter 0)))
  (bind _returnvalue (SaveGame|SaveGametoSlot (Variables|Default|GetSaveRef) (Variables|Default|GetSaveSlotName)))
  (if _returnvalue
    (Development|PrintText (Utilities|Text|FormatText "Saved checkpoint on slot {slotName}" (Variables|Default|GetSaveSlotName)))
    (else
      (Development|PrintText "Error saving file!"))))